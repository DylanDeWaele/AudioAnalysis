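; Actor that turns live constant-Q audio analysis into MIDI notes through a Harmonic Product Spectrum pitch estimate.
; Each Tick it reads the BP_ConstantQAnalyzer spectrum, downsamples it by two and three with interpolation, and multiplies the three spectra.
; When the peak bin changes, that index goes out as a Note On with zero velocity on the MIDI output opened at BeginPlay.
; A note-name printing helper exists but never runs.
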(event `self.ReceiveBeginPlay`
  (`|ExecutionSequence`
    (:`then_0`
      ;[1 1 1] Store the constantQ analyzer
      (bind _returnvalue (`GameplayStatics.GetActorOfClass` "/Game/Analysis/ConstantQ/BP_ConstantQAnalyzer.BP_ConstantQAnalyzer_C"))
      (set `self.ConstantQ` _returnvalue))
    (:`then_1`
      ;[1 1 1] Print out available MIDI devices
      (bind _outmididevices (`MIDIDeviceManager.FindMIDIDevices`))
      (for _array_element _outmididevices
        (`KismetSystemLibrary.PrintString` (`KismetStringLibrary.Concat_StrStr` (`KismetStringLibrary.Conv_IntToString` (break `FoundMIDIDevice` _array_element)) " - " (`.DeviceName` (break `FoundMIDIDevice` _array_element))) true true (struct :`G` 0.66 :`B` 1.0 :`A` 1.0) 10.0)))
    (:`then_2`
      ;[1 1 1] Create MIDI output controller
      (bind _returnvalue_2 (`MIDIDeviceManager.CreateMIDIDeviceOutputController` 0))
      (set `self.MIDIOutput` _returnvalue_2))))

(event `self.ReceiveTick`
  (params (DeltaSeconds :type "Float (single-precision)"))
  (bind _output_get (set `self.Frequencies` (`/Game/Analysis/ConstantQ/BP_ConstantQAnalyzer.CurrentConstantQ` (`self.ConstantQ`))))
  (`|ExecutionSequence`
    (:`then_0`
      ;[1 1 1] Downsample
      (bind _outfrequencies (`self.Downsample` 2 _output_get))
      (set `self.FrequenciesDS2` _outfrequencies))
    (:`then_1`
      (bind _outfrequencies_2 (`self.Downsample` 3 _output_get))
      (set `self.FrequenciesDS3` _outfrequencies_2))
    (:`then_2`
      ;[1 1 1] Multiply spectra, get the fundamental frequency and send MIDI events
      (bind _hpspfrequencies (`self.MultiplySpectra`))
      (bind _indexofmaxvalue (`KismetMathLibrary.MaxOfFloatArray` _hpspfrequencies))
      (if (!= _indexofmaxvalue (`self.LastFundamentalFrequency`))
        (bind _output_get_2 (set `self.LastFundamentalFrequency` _indexofmaxvalue))
        (`self.SendMIDIEvent` _output_get_2)))))

(fn `Downsample`
  (params (Amount :type Integer) (InFrequencies :type "Array of Float (double-precision)"))
  (returns (OutFrequencies :type "Array of Float (double-precision)"))
  (locals (OriginalFrequencies :type "Array of Float (double-precision)") (NewFrequencies :type "Array of Float (double-precision)") (NewArraySize :type Integer) (Index :type Integer) (P :type Integer))
  (bind _originalfrequencies (`local.OriginalFrequencies`))
  (bind _returnvalue (- (`KismetArrayLibrary.Array_Length` (`local.OriginalFrequencies`)) 1))
  ;[1 1 1] Help from: https://stackoverflow.com/questions/31836598/subsampling-an-array-of-numbers
  ;;[1 1 1] Set size
  (bind _output_get (set `local.OriginalFrequencies` InFrequencies))
  (bind _output_get_2 (set `local.NewArraySize` (/ (`KismetArrayLibrary.Array_Length` _output_get) Amount)))
  (for _index (range _output_get_2)
    (`|ExecutionSequence`
      (:`then_0`
        ;;[1 1 1] Compute index
        (set `local.Index` (/ (* _index _returnvalue) (- (`local.NewArraySize`) 1))))
      (:`then_1`
        ;;[1 1 1] Compute P
        (set `local.P` (mod (* _index _returnvalue) (- (`local.NewArraySize`) 1))))
      (:`then_2`
        ;;[1 1 1] Compute value = ((p * a[index + 1]) + ((76 - p) * a[index])) / 76
        (`KismetArrayLibrary.Array_Add` (`local.NewFrequencies`) (/ (+ (* (`local.P`) (`|GetArrayItem` (`local.OriginalFrequencies`) (+ (`local.Index`) 1))) (* (- (- (`local.NewArraySize`) 1) (`local.P`)) (`|GetArrayItem` (`local.OriginalFrequencies`) (`local.Index`)))) (`KismetMathLibrary.Conv_IntToDouble` (- (`local.NewArraySize`) 1)))))))
  ;;[1 1 1] Set last element
  (`KismetArrayLibrary.Array_Set` (`local.NewFrequencies`) (- (`local.NewArraySize`) 1) (`|GetArrayItem` _originalfrequencies (- (`KismetArrayLibrary.Array_Length` _originalfrequencies) 1)))
  (return (`local.NewFrequencies`)))

(fn `MultiplySpectra`
  (returns (HPSPFrequencies :type "Array of Float (double-precision)"))
  (locals (HPSFrequencies :type "Array of Float (double-precision)") (CurrentFrequency :type "Float (double-precision)"))
  (for (_array_element _array_index) (`self.Frequencies`)
    (set `local.CurrentFrequency` _array_element)
    (`|ExecutionSequence`
      (:`then_0`
        ;[1 1 1] Multiply with first downsampled spectrum
        (if (< _array_index (`KismetArrayLibrary.Array_Length` (`self.FrequenciesDS2`)))
          (set `local.CurrentFrequency` (* (`local.CurrentFrequency`) (`|GetArrayItem` (`self.FrequenciesDS2`) _array_index)))))
      (:`then_1`
        ;[1 1 1] Multiply with second downsampled spectrum
        (if (< _array_index (`KismetArrayLibrary.Array_Length` (`self.FrequenciesDS3`)))
          (set `local.CurrentFrequency` (* (`local.CurrentFrequency`) (`|GetArrayItem` (`self.FrequenciesDS3`) _array_index)))))
      (:`then_2`
        ;[1 1 1] Add to final spectrum
        (`KismetArrayLibrary.Array_Add` (`local.HPSFrequencies`) (`local.CurrentFrequency`)))))
  (return (`local.HPSFrequencies`)))

(fn `Print Note`
  (params (Note :type Integer))
  (locals (LocalNote :type Integer) (OctaveNr :type Integer) (NoteString :type String))
  (bind _octavenr (`local.OctaveNr`))
  ;[1 1 1] Calculate correct note string
  (bind _output_get (set `local.LocalNote` (- Note 24)))
  (if (< _output_get 0)
    ;[1 1 1] Special case for A0, A#0/Bb0, B0
    (switch `int` (- Note 21)
      (:`Default`
        (set `local.NoteString` "Not a piano key"))
      (:`0`
        (set `local.NoteString` "A"))
      (:`1`
        (set `local.NoteString` "A#/Bb"))
      (:`2`
        (set `local.NoteString` "B")))
    (`KismetSystemLibrary.PrintString` (`KismetStringLibrary.Concat_StrStr` (`local.NoteString`) "0"))
    (return)
    (else
      (bind _output_get_2 (set `local.OctaveNr` (/ (`local.LocalNote`) 12)))
      (switch `int` (- (`local.LocalNote`) (* _output_get_2 12))
        (:`Default`
          (bind _output_get_3 (set `local.NoteString` "Not a piano key"))
          (`KismetSystemLibrary.PrintString` _output_get_3))
        (:`0`
          (set `local.NoteString` "C")
          (`/Engine/EditorBlueprintResources/StandardMacros.IncrementInt` _octavenr :!label _label
            (:`  `
              (`KismetSystemLibrary.PrintString` (`KismetStringLibrary.Concat_StrStr` (`local.NoteString`) (`KismetStringLibrary.Conv_IntToString` _octavenr)))
              (return))))
        (:`1`
          (set `local.NoteString` "C#/Db")
          (goto _label))
        (:`2`
          (set `local.NoteString` "D")
          (goto _label))
        (:`3`
          (set `local.NoteString` "D#/Eb")
          (goto _label))
        (:`4`
          (set `local.NoteString` "E")
          (goto _label))
        (:`5`
          (set `local.NoteString` "F")
          (goto _label))
        (:`6`
          (set `local.NoteString` "F#/Gb")
          (goto _label))
        (:`7`
          (set `local.NoteString` "G")
          (goto _label))
        (:`8`
          (set `local.NoteString` "G#/Ab")
          (goto _label))
        (:`9`
          (set `local.NoteString` "A")
          (goto _label))
        (:`10`
          (set `local.NoteString` "A#/Bb")
          (goto _label))
        (:`11`
          (set `local.NoteString` "B")
          (goto _label))
        (:`12`
          (set `local.NoteString` "B#/Cb")
          (goto _label))))))

(fn `SendMIDIEvent`
  (params (FrequencyIndex :type Integer))
  (`MIDIDeviceOutputController.SendMIDINoteOn` (`self.MIDIOutput`) 0 FrequencyIndex 0))

(fn `UserConstructionScript`)