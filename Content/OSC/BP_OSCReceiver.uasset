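; Receives OSC messages to remote-control an audio-reactive stage show of fireworks, pyros, static and moving heads, and lasers.
; On BeginPlay it starts an OSC server on a hardcoded IP and port, then routes each message by address path to a Control function with a target class.
; These functions apply the float to all matching actors, setting listener threshold and activation or tilt, zoom and spread toggles; volume targets BP_SoundSource.
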(event `self.ReceiveBeginPlay`
  ;[1 1 1] Initialize OSCServer
  (bind _returnvalue (`OSCManager.CreateOSCServer` "192.168.1.16" 8000 false true "" null))
  (bind _output_get (set `self.OSCServer` _returnvalue))
  (`|ExecutionSequence`
    (:`then_0`
      (clear `OSCServer.OnOscMessageReceived` _output_get))
    (:`then_1`
      (add `OSCServer.OnOscMessageReceived` _output_get (delegate `OnOscMessageReceived`)))))

(event `OnOscMessageReceived`
  (params (Message :type "OSCMessage Structure (by ref)") (IPAddress :type String) (Port :type Integer))
  ;[1 1 1] Check what to do with the message
  (bind _returnvalue (`OSCManager.GetOSCMessageAddress` Message))
  (bind _returnvalue_2 (`OSCManager.GetOSCAddressFullPath` _returnvalue))
  (switch `string` _returnvalue_2
    (:`/1/FireworksTreshold`
      (`self.ControlTreshold` Message "/Game/DMX/BP_MyFireworksLauncher.BP_MyFireworksLauncher_C"))
    (:`/1/FireworksActive`
      (`self.ControlActive` Message "/Game/DMX/BP_MyFireworksLauncher.BP_MyFireworksLauncher_C"))
    (:`/1/PyrosTreshold`
      (`self.ControlTreshold` Message "/Game/DMX/BP_MyPyroModule.BP_MyPyroModule_C"))
    (:`/1/PyrosActive`
      (`self.ControlActive` Message "/Game/DMX/BP_MyPyroModule.BP_MyPyroModule_C"))
    (:`/1/StaticLowTreshold`
      (`self.ControlTreshold` Message "/Game/DMX/StaticHeads/BP_LowFreqStaticHead.BP_LowFreqStaticHead_C"))
    (:`/1/StaticMidTreshold`
      (`self.ControlTreshold` Message "/Game/DMX/StaticHeads/BP_MidFreqStaticHead.BP_MidFreqStaticHead_C"))
    (:`/1/StaticHighTreshold`
      (`self.ControlTreshold` Message "/Game/DMX/StaticHeads/BP_HighFreqStaticHead.BP_HighFreqStaticHead_C"))
    (:`/1/StaticLowActive`
      (`self.ControlActive` Message "/Game/DMX/StaticHeads/BP_LowFreqStaticHead.BP_LowFreqStaticHead_C"))
    (:`/1/StaticMidActive`
      (`self.ControlActive` Message "/Game/DMX/StaticHeads/BP_MidFreqStaticHead.BP_MidFreqStaticHead_C"))
    (:`/1/StaticHighActive`
      (`self.ControlActive` Message "/Game/DMX/StaticHeads/BP_HighFreqStaticHead.BP_HighFreqStaticHead_C"))
    (:`/1/MovingLowTreshold`
      (`self.ControlTreshold` Message "/Game/DMX/MovingHeads/BP_LowFreqsMovingHead.BP_LowFreqsMovingHead_C"))
    (:`/1/MovingMidTreshold`
      (`self.ControlTreshold` Message "/Game/DMX/MovingHeads/BP_MidFreqsMovingHead.BP_MidFreqsMovingHead_C"))
    (:`/1/MovingHighTreshold`
      (`self.ControlTreshold` Message "/Game/DMX/MovingHeads/BP_HighFreqsMovingHead.BP_HighFreqsMovingHead_C"))
    (:`/1/MovingLowActive`
      (`self.ControlActive` Message "/Game/DMX/MovingHeads/BP_LowFreqsMovingHead.BP_LowFreqsMovingHead_C"))
    (:`/1/MovingMidActive`
      (`self.ControlActive` Message "/Game/DMX/MovingHeads/BP_MidFreqsMovingHead.BP_MidFreqsMovingHead_C"))
    (:`/1/MovingHighActive`
      (`self.ControlActive` Message "/Game/DMX/MovingHeads/BP_HighFreqsMovingHead.BP_HighFreqsMovingHead_C"))
    (:`/1/MovingLowTilt`
      (`self.ControlTilt` Message "/Game/DMX/MovingHeads/BP_LowFreqsMovingHead.BP_LowFreqsMovingHead_C"))
    (:`/1/MovingMidTilt`
      (`self.ControlTilt` Message "/Game/DMX/MovingHeads/BP_MidFreqsMovingHead.BP_MidFreqsMovingHead_C"))
    (:`/1/MovingHighTilt`
      (`self.ControlTilt` Message "/Game/DMX/MovingHeads/BP_HighFreqsMovingHead.BP_HighFreqsMovingHead_C"))
    (:`/1/MovingLowZoom`
      (`self.ControlZoom` Message "/Game/DMX/MovingHeads/BP_LowFreqsMovingHead.BP_LowFreqsMovingHead_C"))
    (:`/1/MovingMidZoom`
      (`self.ControlZoom` Message "/Game/DMX/MovingHeads/BP_MidFreqsMovingHead.BP_MidFreqsMovingHead_C"))
    (:`/1/MovingHighZoom`
      (`self.ControlZoom` Message "/Game/DMX/MovingHeads/BP_HighFreqsMovingHead.BP_HighFreqsMovingHead_C"))
    (:`/1/LaserLowTreshold`
      (`self.ControlTreshold` Message "/Game/DMX/Lasers/BP_LowFreqLaser.BP_LowFreqLaser_C"))
    (:`/1/LaserMidTreshold`
      (`self.ControlTreshold` Message "/Game/DMX/Lasers/BP_MidFreqLaser.BP_MidFreqLaser_C"))
    (:`/1/LaserHighTreshold`
      (`self.ControlTreshold` Message "/Game/DMX/Lasers/BP_HighFreqLaser.BP_HighFreqLaser_C"))
    (:`/1/LaserLowActive`
      (`self.ControlActive` Message "/Game/DMX/Lasers/BP_LowFreqLaser.BP_LowFreqLaser_C"))
    (:`/1/LaserMidActive`
      (`self.ControlActive` Message "/Game/DMX/Lasers/BP_MidFreqLaser.BP_MidFreqLaser_C"))
    (:`/1/LaserHighActive`
      (`self.ControlActive` Message "/Game/DMX/Lasers/BP_HighFreqLaser.BP_HighFreqLaser_C"))
    (:`/1/LaserLowSpread`
      (`self.ControlSpread` Message "/Game/DMX/Lasers/BP_LowFreqLaser.BP_LowFreqLaser_C"))
    (:`/1/LaserMidSpread`
      (`self.ControlSpread` Message "/Game/DMX/Lasers/BP_MidFreqLaser.BP_MidFreqLaser_C"))
    (:`/1/LaserHighSpread`
      (`self.ControlSpread` Message "/Game/DMX/Lasers/BP_HighFreqLaser.BP_HighFreqLaser_C"))
    (:`/1/Volume`
      (`self.ControlVolume` Message))))

(fn `ControlActive`
  (params (Message :type "OSCMessage Structure") (`Actor Class` :type "Actor Class Reference"))
  (bind (_value _returnvalue) (`OSCManager.GetFloat` Message))
  (if _returnvalue
    (bind _outactors (`GameplayStatics.GetAllActorsOfClass` `Actor Class`))
    (for _array_element _outactors
      ;[1 1 1] Choose with which class to continue on
      (bind _asbp_my_fireworks_launcher (cast `/Game/DMX/BP_MyFireworksLauncher` _array_element)
        (:`then`
          (bind _returnvalue_2 (`KismetMathLibrary.FTrunc` _value))
          (switch `int` _returnvalue_2
            (:`0`
              (bind _constantqlistenercomponent (`/Game/DMX/BP_MyFireworksLauncher.ConstantQListenerComponent` _asbp_my_fireworks_launcher))
              (`ActorComponent.Deactivate` _constantqlistenercomponent))
            (:`1`
              (`ActorComponent.Activate` _constantqlistenercomponent false))))
        (:`CastFailed`
          (bind _asbp_my_laser_module (cast `/Game/DMX/Lasers/BP_MyLaserModule` _array_element)
            (:`then`
              (switch `int` _returnvalue_2
                (:`0`
                  (bind _constantqlistenercomponent_2 (`/Game/DMX/Lasers/BP_MyLaserModule.ConstantQListenerComponent` _asbp_my_laser_module))
                  (`ActorComponent.Deactivate` _constantqlistenercomponent_2))
                (:`1`
                  (`ActorComponent.Activate` _constantqlistenercomponent_2 false))))
            (:`CastFailed`
              (bind _asbp_my_moving_head (cast `/Game/DMX/MovingHeads/BP_MyMovingHead` _array_element)
                (:`then`
                  (switch `int` _returnvalue_2
                    (:`0`
                      (bind _constantqlistenercomponent_3 (`/Game/DMX/MovingHeads/BP_MyMovingHead.ConstantQListenerComponent` _asbp_my_moving_head))
                      (`ActorComponent.Deactivate` _constantqlistenercomponent_3))
                    (:`1`
                      (`ActorComponent.Activate` _constantqlistenercomponent_3 false))))
                (:`CastFailed`
                  (bind _asbp_my_pyro_module (cast `/Game/DMX/BP_MyPyroModule` _array_element)
                    (:`then`
                      (switch `int` _returnvalue_2
                        (:`0`
                          (bind _constantqlistenercomponent_4 (`/Game/DMX/BP_MyPyroModule.ConstantQListenerComponent` _asbp_my_pyro_module))
                          (`ActorComponent.Deactivate` _constantqlistenercomponent_4))
                        (:`1`
                          (`ActorComponent.Activate` _constantqlistenercomponent_4 false))))
                    (:`CastFailed`
                      (bind _asbp_my_static_head (cast `/Game/DMX/StaticHeads/BP_MyStaticHead` _array_element))
                      (switch `int` _returnvalue_2
                        (:`0`
                          (bind _constantqlistenercomponent_5 (`/Game/DMX/StaticHeads/BP_MyStaticHead.ConstantQListenerComponent` _asbp_my_static_head))
                          (`ActorComponent.Deactivate` _constantqlistenercomponent_5))
                        (:`1`
                          (`ActorComponent.Activate` _constantqlistenercomponent_5 false))))))))))))
    (else
      (`KismetSystemLibrary.PrintString` "Failed to get value from OSC message" true true (struct :`R` 1.0 :`G` 0.031819 :`A` 1.0) 5.0))))

(fn `ControlSpread`
  (params (Message :type "OSCMessage Structure") (ActorClass :type "Actor Class Reference"))
  (bind (_value _returnvalue) (`OSCManager.GetFloat` Message))
  (if _returnvalue
    (bind _outactors (`GameplayStatics.GetAllActorsOfClass` ActorClass))
    (for _array_element _outactors
      ;[1 1 1] Decide on which frequencies to apply it on
      (bind _asbp_low_freq_laser (cast `/Game/DMX/Lasers/BP_LowFreqLaser` _array_element)
        (:`then`
          (bind _returnvalue_2 (`KismetMathLibrary.FTrunc` _value))
          (switch `int` _returnvalue_2
            (:`0`
              (set `/Game/DMX/Lasers/BP_MyLaserModule.UseSpread` false _asbp_low_freq_laser))
            (:`1`
              (set `/Game/DMX/Lasers/BP_MyLaserModule.UseSpread` true _asbp_low_freq_laser))))
        (:`CastFailed`
          (bind _asbp_mid_freq_laser (cast `/Game/DMX/Lasers/BP_MidFreqLaser` _array_element)
            (:`then`
              (switch `int` _returnvalue_2
                (:`0`
                  (set `/Game/DMX/Lasers/BP_MyLaserModule.UseSpread` false _asbp_mid_freq_laser))
                (:`1`
                  (set `/Game/DMX/Lasers/BP_MyLaserModule.UseSpread` true _asbp_mid_freq_laser))))
            (:`CastFailed`
              (bind _asbp_high_freq_laser (cast `/Game/DMX/Lasers/BP_HighFreqLaser` _array_element))
              (switch `int` _returnvalue_2
                (:`0`
                  (set `/Game/DMX/Lasers/BP_MyLaserModule.UseSpread` false _asbp_high_freq_laser))
                (:`1`
                  (set `/Game/DMX/Lasers/BP_MyLaserModule.UseSpread` true _asbp_high_freq_laser))))))))
    (else
      (`KismetSystemLibrary.PrintString` "Failed to get value from OSC message" true true (struct :`R` 1.0 :`G` 0.031819 :`A` 1.0) 5.0))))

(fn `ControlTilt`
  (params (Message :type "OSCMessage Structure") (ActorClass :type "Actor Class Reference"))
  (bind (_value _returnvalue) (`OSCManager.GetFloat` Message))
  (if _returnvalue
    (bind _outactors (`GameplayStatics.GetAllActorsOfClass` ActorClass))
    (for _array_element _outactors
      ;[1 1 1] Decide on which frequencies to apply it on
      (bind _asbp_low_freqs_moving_head (cast `/Game/DMX/MovingHeads/BP_LowFreqsMovingHead` _array_element)
        (:`then`
          (bind _returnvalue_2 (`KismetMathLibrary.FTrunc` _value))
          (switch `int` _returnvalue_2
            (:`0`
              (set `/Game/DMX/MovingHeads/BP_MyMovingHead.UseTilt` false _asbp_low_freqs_moving_head))
            (:`1`
              (set `/Game/DMX/MovingHeads/BP_MyMovingHead.UseTilt` true _asbp_low_freqs_moving_head))))
        (:`CastFailed`
          (bind _asbp_mid_freqs_moving_head (cast `/Game/DMX/MovingHeads/BP_MidFreqsMovingHead` _array_element)
            (:`then`
              (switch `int` _returnvalue_2
                (:`0`
                  (set `/Game/DMX/MovingHeads/BP_MyMovingHead.UseTilt` false _asbp_mid_freqs_moving_head))
                (:`1`
                  (set `/Game/DMX/MovingHeads/BP_MyMovingHead.UseTilt` true _asbp_mid_freqs_moving_head))))
            (:`CastFailed`
              (bind _asbp_high_freqs_moving_head (cast `/Game/DMX/MovingHeads/BP_HighFreqsMovingHead` _array_element))
              (switch `int` _returnvalue_2
                (:`0`
                  (set `/Game/DMX/MovingHeads/BP_MyMovingHead.UseTilt` false _asbp_high_freqs_moving_head))
                (:`1`
                  (set `/Game/DMX/MovingHeads/BP_MyMovingHead.UseTilt` true _asbp_high_freqs_moving_head))))))))
    (else
      (`KismetSystemLibrary.PrintString` "Failed to get value from OSC message" true true (struct :`R` 1.0 :`G` 0.031819 :`A` 1.0) 5.0))))

(fn `ControlTreshold`
  (params (Message :type "OSCMessage Structure") (ActorClass :type "Actor Class Reference"))
  (bind (_value _returnvalue) (`OSCManager.GetFloat` Message))
  (if _returnvalue
    (bind _outactors (`GameplayStatics.GetAllActorsOfClass` ActorClass))
    (for _array_element _outactors
      ;[1 1 1] Choose with which class to continue on
      (bind _asbp_my_fireworks_launcher (cast `/Game/DMX/BP_MyFireworksLauncher` _array_element)
        (:`then`
          (set `/Game/Components/BP_ConstantQListenerComponent.Treshold` _value (`/Game/DMX/BP_MyFireworksLauncher.ConstantQListenerComponent` _asbp_my_fireworks_launcher)))
        (:`CastFailed`
          (bind _asbp_my_laser_module (cast `/Game/DMX/Lasers/BP_MyLaserModule` _array_element)
            (:`then`
              (set `/Game/Components/BP_ConstantQListenerComponent.Treshold` _value (`/Game/DMX/Lasers/BP_MyLaserModule.ConstantQListenerComponent` _asbp_my_laser_module)))
            (:`CastFailed`
              (bind _asbp_my_moving_head (cast `/Game/DMX/MovingHeads/BP_MyMovingHead` _array_element)
                (:`then`
                  (set `/Game/Components/BP_ConstantQListenerComponent.Treshold` _value (`/Game/DMX/MovingHeads/BP_MyMovingHead.ConstantQListenerComponent` _asbp_my_moving_head)))
                (:`CastFailed`
                  (bind _asbp_my_pyro_module (cast `/Game/DMX/BP_MyPyroModule` _array_element)
                    (:`then`
                      (set `/Game/Components/BP_ConstantQListenerComponent.Treshold` _value (`/Game/DMX/BP_MyPyroModule.ConstantQListenerComponent` _asbp_my_pyro_module)))
                    (:`CastFailed`
                      (bind _asbp_my_static_head (cast `/Game/DMX/StaticHeads/BP_MyStaticHead` _array_element))
                      (set `/Game/Components/BP_ConstantQListenerComponent.Treshold` _value (`/Game/DMX/StaticHeads/BP_MyStaticHead.ConstantQListenerComponent` _asbp_my_static_head)))))))))))
    (else
      (`KismetSystemLibrary.PrintString` "Failed to get value from OSC message" true true (struct :`R` 1.0 :`G` 0.031819 :`A` 1.0) 5.0))))

(fn `ControlVolume`
  (params (Message :type "OSCMessage Structure"))
  (bind (_value _returnvalue) (`OSCManager.GetFloat` Message))
  (if _returnvalue
    (bind _returnvalue_2 (`GameplayStatics.GetActorOfClass` "/Game/Sounds/BP_SoundSource.BP_SoundSource_C"))
    (`AudioComponent.SetVolumeMultiplier` (`/Game/Sounds/BP_SoundSource.AudioComponent` _returnvalue_2) _value)
    (else
      (`KismetSystemLibrary.PrintString` "Failed to get value from OSC message" true true (struct :`R` 1.0 :`G` 0.031819 :`A` 1.0) 5.0))))

(fn `ControlZoom`
  (params (Message :type "OSCMessage Structure") (ActorClass :type "Actor Class Reference"))
  (bind (_value _returnvalue) (`OSCManager.GetFloat` Message))
  (if _returnvalue
    (bind _outactors (`GameplayStatics.GetAllActorsOfClass` ActorClass))
    (for _array_element _outactors
      ;[1 1 1] Decide on which frequencies to apply it on
      (bind _asbp_low_freqs_moving_head (cast `/Game/DMX/MovingHeads/BP_LowFreqsMovingHead` _array_element)
        (:`then`
          (bind _returnvalue_2 (`KismetMathLibrary.FTrunc` _value))
          (switch `int` _returnvalue_2
            (:`0`
              (set `/Game/DMX/MovingHeads/BP_MyMovingHead.UseZoom` false _asbp_low_freqs_moving_head))
            (:`1`
              (set `/Game/DMX/MovingHeads/BP_MyMovingHead.UseZoom` true _asbp_low_freqs_moving_head))))
        (:`CastFailed`
          (bind _asbp_mid_freqs_moving_head (cast `/Game/DMX/MovingHeads/BP_MidFreqsMovingHead` _array_element)
            (:`then`
              (switch `int` _returnvalue_2
                (:`0`
                  (set `/Game/DMX/MovingHeads/BP_MyMovingHead.UseZoom` false _asbp_mid_freqs_moving_head))
                (:`1`
                  (set `/Game/DMX/MovingHeads/BP_MyMovingHead.UseZoom` true _asbp_mid_freqs_moving_head))))
            (:`CastFailed`
              (bind _asbp_high_freqs_moving_head (cast `/Game/DMX/MovingHeads/BP_HighFreqsMovingHead` _array_element))
              (switch `int` _returnvalue_2
                (:`0`
                  (set `/Game/DMX/MovingHeads/BP_MyMovingHead.UseZoom` false _asbp_high_freqs_moving_head))
                (:`1`
                  (set `/Game/DMX/MovingHeads/BP_MyMovingHead.UseZoom` true _asbp_high_freqs_moving_head))))))))
    (else
      (`KismetSystemLibrary.PrintString` "Failed to get value from OSC message" true true (struct :`R` 1.0 :`G` 0.031819 :`A` 1.0) 5.0))))

(fn `UserConstructionScript`)