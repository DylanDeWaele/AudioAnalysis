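; Sends OSC float messages to an Android controller, mirroring the state of a music-reactive stage show.
; On BeginPlay it creates a client with a hardcoded IP and port, caches the audio analyzers, and sends starting active, threshold, option and volume values from fireworks, pyro, light, laser and sound actors.
; Each tick it streams loudness, low/mid/high Constant-Q band averages and onset strength.
; Actors are found with GetActorOfClass, so only one instance per class is read.
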(event `self.ReceiveBeginPlay`
  ;[1 1 1] Initialize OSCClient and analyzer classes
  (`|ExecutionSequence`
    (:`then_0`
      (bind _returnvalue (`OSCManager.CreateOSCClient` "192.168.1.2" 9000 "" null))
      (set `self.OSCClient` _returnvalue))
    (:`then_1`
      (bind _returnvalue_2 (`GameplayStatics.GetActorOfClass` "/Game/Analysis/Loudness/BP_LoudnessAnalyzer.BP_LoudnessAnalyzer_C"))
      (set `self.LoudnessAnalyzer` _returnvalue_2))
    (:`then_2`
      (bind _returnvalue_3 (`GameplayStatics.GetActorOfClass` "/Game/Analysis/ConstantQ/BP_ConstantQAnalyzer.BP_ConstantQAnalyzer_C"))
      (set `self.ConstantQAnalyzer` _returnvalue_3))
    (:`then_3`
      (bind _returnvalue_4 (`GameplayStatics.GetActorOfClass` "/Game/Analysis/Onset/BP_OnsetAnalyzer.BP_OnsetAnalyzer_C"))
      (set `self.OnsetAnalyzer` _returnvalue_4))
    (:`then_4`
      (`self.SendStartingValues`))))

(event `self.ReceiveTick`
  (params (DeltaSeconds :type "Float (single-precision)"))
  ;[1 1 1] Send OSC Messages to the android controller
  (`|ExecutionSequence`
    (:`then_0`
      (`self.SendLoudness`))
    (:`then_1`
      (`self.SendFrequenciesAverage` 0))
    (:`then_2`
      (`self.SendFrequenciesAverage` 1))
    (:`then_3`
      (`self.SendFrequenciesAverage` 2))
    (:`then_4`
      (`self.SendOnset`))))

(fn `SendAssetStartingValues`
  (params (Active :type Boolean) (Treshold :type "Float (double-precision)") (Name :type String))
  (bind _returnvalue (`KismetStringLibrary.Concat_StrStr` Name "Active"))
  (`self.SendOSCFloat` (`KismetStringLibrary.Concat_StrStr` Name "Treshold") Treshold)
  (if Active
    (`self.SendOSCFloat` _returnvalue 1.0)
    (else
      (`self.SendOSCFloat` _returnvalue))))

(fn `SendFrequenciesAverage`
  (params (FrequencyRange :type Integer))
  (locals (Address :type String))
  (bind _constantqanalyzer (`self.ConstantQAnalyzer`))
  (switch `int` FrequencyRange
    (:`0`
      (set `local.Address` "/1/LowFreq"))
    (:`1`
      (set `local.Address` "/1/MidFreq"))
    (:`2`
      (set `local.Address` "/1/HighFreq")))
  (bind _requestedfrequencies (`/Game/Analysis/ConstantQ/BP_ConstantQAnalyzer.GetFrequencyRange` _constantqanalyzer FrequencyRange))
  (bind _average (`/Game/Analysis/ConstantQ/BP_ConstantQAnalyzer.GetFrequencyRangeAverage` _constantqanalyzer _requestedfrequencies))
  (`self.SendOSCFloat` (`local.Address`) _average))

(fn `SendLoudness`
  (locals (OSCMessage :type "OSCMessage Structure"))
  (`self.SendOSCFloat` "/1/Loudness" (`/Game/Analysis/Loudness/BP_LoudnessAnalyzer.CurrentLoudness` (`self.LoudnessAnalyzer`))))

(fn `SendOnset`
  (`self.SendOSCFloat` "/1/Onset" (`/Game/Analysis/Onset/BP_OnsetAnalyzer.CurrentOnsetStrength` (`self.OnsetAnalyzer`))))

(fn `SendOSCFloat`
  (params (Address :type String) (Value :type "Float (double-precision)"))
  ;[1 1 1] Send a float value to a given OSC address
  (bind _returnvalue (`OSCManager.ConvertStringToOSCAddress` Address))
  (bind _returnvalue_2 (`OSCManager.SetOSCMessageAddress` (make `OSCMessage`) _returnvalue))
  (bind _returnvalue_3 (`OSCManager.AddFloat` _returnvalue_2 Value))
  (`OSCClient.SendOSCMessage` (`self.OSCClient`) _returnvalue_3))

(fn `SendStartingValues`
  (`|ExecutionSequence`
    (:`then_0`
      ;[1 1 1] Send fireworks starting values
      (bind _returnvalue (`GameplayStatics.GetActorOfClass` "/Game/DMX/BP_MyFireworksLauncher.BP_MyFireworksLauncher_C"))
      (bind _constantqlistenercomponent (`/Game/DMX/BP_MyFireworksLauncher.ConstantQListenerComponent` _returnvalue))
      (`self.SendAssetStartingValues` (`ActorComponent.IsActive` _constantqlistenercomponent) (`/Game/Components/BP_ConstantQListenerComponent.Treshold` _constantqlistenercomponent) "/1/Fireworks"))
    (:`then_1`
      ;[1 1 1] Send Pyros starting values
      (bind _returnvalue_2 (`GameplayStatics.GetActorOfClass` "/Game/DMX/BP_MyPyroModule.BP_MyPyroModule_C"))
      (bind _constantqlistenercomponent_2 (`/Game/DMX/BP_MyPyroModule.ConstantQListenerComponent` _returnvalue_2))
      (`self.SendAssetStartingValues` (`ActorComponent.IsActive` _constantqlistenercomponent_2) (`/Game/Components/BP_ConstantQListenerComponent.Treshold` _constantqlistenercomponent_2) "/1/Pyros"))
    (:`then_2`
      ;[1 1 1] Send static lows starting values
      (bind _returnvalue_3 (`GameplayStatics.GetActorOfClass` "/Game/DMX/StaticHeads/BP_LowFreqStaticHead.BP_LowFreqStaticHead_C"))
      (bind _constantqlistenercomponent_3 (`/Game/DMX/StaticHeads/BP_MyStaticHead.ConstantQListenerComponent` _returnvalue_3))
      (`self.SendAssetStartingValues` (`ActorComponent.IsActive` _constantqlistenercomponent_3) (`/Game/Components/BP_ConstantQListenerComponent.Treshold` _constantqlistenercomponent_3) "/1/StaticLow"))
    (:`then_3`
      ;[1 1 1] Send static mids starting values
      (bind _returnvalue_4 (`GameplayStatics.GetActorOfClass` "/Game/DMX/StaticHeads/BP_MidFreqStaticHead.BP_MidFreqStaticHead_C"))
      (bind _constantqlistenercomponent_4 (`/Game/DMX/StaticHeads/BP_MyStaticHead.ConstantQListenerComponent` _returnvalue_4))
      (`self.SendAssetStartingValues` (`ActorComponent.IsActive` _constantqlistenercomponent_4) (`/Game/Components/BP_ConstantQListenerComponent.Treshold` _constantqlistenercomponent_4) "/1/StaticMid"))
    (:`then_4`
      ;[1 1 1] Send static highs starting values
      (bind _returnvalue_5 (`GameplayStatics.GetActorOfClass` "/Game/DMX/StaticHeads/BP_HighFreqStaticHead.BP_HighFreqStaticHead_C"))
      (bind _constantqlistenercomponent_5 (`/Game/DMX/StaticHeads/BP_MyStaticHead.ConstantQListenerComponent` _returnvalue_5))
      (`self.SendAssetStartingValues` (`ActorComponent.IsActive` _constantqlistenercomponent_5) (`/Game/Components/BP_ConstantQListenerComponent.Treshold` _constantqlistenercomponent_5) "/1/StaticHigh"))
    (:`then_5`
      ;[1 1 1] Send moving lows starting values
      (bind _returnvalue_6 (`GameplayStatics.GetActorOfClass` "/Game/DMX/MovingHeads/BP_LowFreqsMovingHead.BP_LowFreqsMovingHead_C"))
      (`|ExecutionSequence`
        (:`then_0`
          (bind _constantqlistenercomponent_6 (`/Game/DMX/MovingHeads/BP_MyMovingHead.ConstantQListenerComponent` _returnvalue_6))
          (`self.SendAssetStartingValues` (`ActorComponent.IsActive` _constantqlistenercomponent_6) (`/Game/Components/BP_ConstantQListenerComponent.Treshold` _constantqlistenercomponent_6) "/1/MovingLow"))
        (:`then_1`
          (if (`/Game/DMX/MovingHeads/BP_MyMovingHead.UseTilt` _returnvalue_6)
            (`self.SendOSCFloat` "/1/MovingLowTilt" 1.0)
            (else
              (`self.SendOSCFloat` "/1/MovingLowTilt"))))
        (:`then_2`
          (if (`/Game/DMX/MovingHeads/BP_MyMovingHead.UseZoom` _returnvalue_6)
            (`self.SendOSCFloat` "/1/MovingLowZoom" 1.0)
            (else
              (`self.SendOSCFloat` "/1/MovingLowZoom"))))))
    (:`then_6`
      ;[1 1 1] Send moving Mids starting values
      (bind _returnvalue_7 (`GameplayStatics.GetActorOfClass` "/Game/DMX/MovingHeads/BP_MidFreqsMovingHead.BP_MidFreqsMovingHead_C"))
      (`|ExecutionSequence`
        (:`then_0`
          (bind _constantqlistenercomponent_7 (`/Game/DMX/MovingHeads/BP_MyMovingHead.ConstantQListenerComponent` _returnvalue_7))
          (`self.SendAssetStartingValues` (`ActorComponent.IsActive` _constantqlistenercomponent_7) (`/Game/Components/BP_ConstantQListenerComponent.Treshold` _constantqlistenercomponent_7) "/1/MovingMid"))
        (:`then_1`
          (if (`/Game/DMX/MovingHeads/BP_MyMovingHead.UseTilt` _returnvalue_7)
            (`self.SendOSCFloat` "/1/MovingMidTilt" 1.0)
            (else
              (`self.SendOSCFloat` "/1/MovingMidTilt"))))
        (:`then_2`
          (if (`/Game/DMX/MovingHeads/BP_MyMovingHead.UseZoom` _returnvalue_7)
            (`self.SendOSCFloat` "/1/MovingMidZoom" 1.0)
            (else
              (`self.SendOSCFloat` "/1/MovingMidZoom"))))))
    (:`then_7`
      ;[1 1 1] Send moving Highs starting values
      (bind _returnvalue_8 (`GameplayStatics.GetActorOfClass` "/Game/DMX/MovingHeads/BP_HighFreqsMovingHead.BP_HighFreqsMovingHead_C"))
      (`|ExecutionSequence`
        (:`then_0`
          (bind _constantqlistenercomponent_8 (`/Game/DMX/MovingHeads/BP_MyMovingHead.ConstantQListenerComponent` _returnvalue_8))
          (`self.SendAssetStartingValues` (`ActorComponent.IsActive` _constantqlistenercomponent_8) (`/Game/Components/BP_ConstantQListenerComponent.Treshold` _constantqlistenercomponent_8) "/1/MovingHigh"))
        (:`then_1`
          (if (`/Game/DMX/MovingHeads/BP_MyMovingHead.UseTilt` _returnvalue_8)
            (`self.SendOSCFloat` "/1/MovingHighTilt" 1.0)
            (else
              (`self.SendOSCFloat` "/1/MovingHighTilt"))))
        (:`then_2`
          (if (`/Game/DMX/MovingHeads/BP_MyMovingHead.UseZoom` _returnvalue_8)
            (`self.SendOSCFloat` "/1/MovingHighZoom" 1.0)
            (else
              (`self.SendOSCFloat` "/1/MovingHighZoom"))))))
    (:`then_8`
      ;[1 1 1] Send laser low starting values
      (bind _returnvalue_9 (`GameplayStatics.GetActorOfClass` "/Game/DMX/Lasers/BP_LowFreqLaser.BP_LowFreqLaser_C"))
      (`|ExecutionSequence`
        (:`then_0`
          (bind _constantqlistenercomponent_9 (`/Game/DMX/Lasers/BP_MyLaserModule.ConstantQListenerComponent` _returnvalue_9))
          (`self.SendAssetStartingValues` (`ActorComponent.IsActive` _constantqlistenercomponent_9) (`/Game/Components/BP_ConstantQListenerComponent.Treshold` _constantqlistenercomponent_9) "/1/LaserLow"))
        (:`then_1`
          (if (`/Game/DMX/Lasers/BP_MyLaserModule.UseSpread` _returnvalue_9)
            (`self.SendOSCFloat` "/1/LaserLowSpread" 1.0)
            (else
              (`self.SendOSCFloat` "/1/LaserLowSpread"))))))
    (:`then_9`
      ;[1 1 1] Send laser mid starting values
      (bind _returnvalue_10 (`GameplayStatics.GetActorOfClass` "/Game/DMX/Lasers/BP_MidFreqLaser.BP_MidFreqLaser_C"))
      (`|ExecutionSequence`
        (:`then_0`
          (bind _constantqlistenercomponent_10 (`/Game/DMX/Lasers/BP_MyLaserModule.ConstantQListenerComponent` _returnvalue_10))
          (`self.SendAssetStartingValues` (`ActorComponent.IsActive` _constantqlistenercomponent_10) (`/Game/Components/BP_ConstantQListenerComponent.Treshold` _constantqlistenercomponent_10) "/1/LaserMid"))
        (:`then_1`
          (if (`/Game/DMX/Lasers/BP_MyLaserModule.UseSpread` _returnvalue_10)
            (`self.SendOSCFloat` "/1/LaserMidSpread" 1.0)
            (else
              (`self.SendOSCFloat` "/1/LaserMidSpread"))))))
    (:`then_10`
      ;[1 1 1] Send laser high starting values
      (bind _returnvalue_11 (`GameplayStatics.GetActorOfClass` "/Game/DMX/Lasers/BP_HighFreqLaser.BP_HighFreqLaser_C"))
      (`|ExecutionSequence`
        (:`then_0`
          (bind _constantqlistenercomponent_11 (`/Game/DMX/Lasers/BP_MyLaserModule.ConstantQListenerComponent` _returnvalue_11))
          (`self.SendAssetStartingValues` (`ActorComponent.IsActive` _constantqlistenercomponent_11) (`/Game/Components/BP_ConstantQListenerComponent.Treshold` _constantqlistenercomponent_11) "/1/LaserHigh"))
        (:`then_1`
          (if (`/Game/DMX/Lasers/BP_MyLaserModule.UseSpread` _returnvalue_11)
            (`self.SendOSCFloat` "/1/LaserHighSpread" 1.0)
            (else
              (`self.SendOSCFloat` "/1/LaserHighSpread"))))))
    (:`then_11`
      ;[1 1 1] Send volume starting values
      (bind _returnvalue_12 (`GameplayStatics.GetActorOfClass` "/Game/Sounds/BP_SoundSource.BP_SoundSource_C"))
      (`self.SendOSCFloat` "/1/Volume" (`AudioComponent.VolumeMultiplier` (`/Game/Sounds/BP_SoundSource.AudioComponent` _returnvalue_12))))))

(fn `UserConstructionScript`)