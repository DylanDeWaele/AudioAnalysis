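; Actor that visualizes the loudness of a sound as a cube, synced to playback.
; On BeginPlay it assigns the LoudnessNRT asset's sound to the level's BP_SoundSource, binds to its playback-percent event and plays it.
; Each update converts percent to seconds and samples the precomputed normalized loudness of channel 0.
; That value drives the cube's Z scale and the "Loudness" parameter on a dynamic MI_Loudness instance created in construction.
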(event `self.ReceiveBeginPlay`
  (bind _soundsourceaudiocomponent (`self.SoundSourceAudioComponent`))
  (bind _sound (`AudioAnalyzerNRT.Sound` (`self.LoudnessNRT`)))
  (`|ExecutionSequence`
    (:`then_0`
      ;[1 1 1] Initialize duration with the duration of the current sound being analyzed and set the sound inside the sound source
      (bind _returnvalue (`GameplayStatics.GetActorOfClass` "/Game/Sounds/BP_SoundSource.BP_SoundSource_C"))
      (bind _output_get (set `self.SoundSourceAudioComponent` (`/Game/Sounds/BP_SoundSource.AudioComponent` _returnvalue)))
      (`AudioComponent.SetSound` _output_get _sound)
      (set `self.Duration` (`SoundBase.Duration` _sound)))
    (:`then_1`
      ;[1 1 1] Bind event to audio playback event
      (add `AudioComponent.OnAudioPlaybackPercent` _soundsourceaudiocomponent (delegate `OnAudioPlaybackPercent_Event_0`))
      (`AudioComponent.Play` _soundsourceaudiocomponent 0.0))))

(event `OnAudioPlaybackPercent_Event_0`
  (params (PlayingSoundWave :type "SoundWave Object Reference") (PlaybackPercent :type "Float (double-precision)"))
  (bind _cube (`self.Cube`))
  (bind (_returnvalue_x _returnvalue_y) (`KismetMathLibrary.BreakVector` (`SceneComponent.K2_GetComponentScale` _cube)))
  ;[1 1 1] Get loudness result the NRT analyzer
  (bind _output_get (set `self.CurrentLoudness` (`LoudnessNRT.GetNormalizedChannelLoudnessAtTime` (`self.LoudnessNRT`) (* PlaybackPercent (`self.Duration`)) 0)))
  ;[1 1 1] Set material parameter
  (`MaterialInstanceDynamic.SetScalarParameterValue` (`self.Dynamic Material`) "Loudness" _output_get)
  ;[1 1 1] Set scale
  (`SceneComponent.SetWorldScale3D` _cube (`KismetMathLibrary.MakeVector` _returnvalue_x _returnvalue_y (* (`self.CurrentLoudness`) 5.0))))

(fn `UserConstructionScript`
  ;[1 1 1] Create and set dynamic material instance on the cube of this object
  (bind _returnvalue (`KismetMaterialLibrary.CreateDynamicMaterialInstance` "/Game/Materials/Instances/MI_Loudness.MI_Loudness"))
  (bind _output_get (set `self.Dynamic Material` _returnvalue))
  (`PrimitiveComponent.SetMaterial` (`self.Cube`) 0 _output_get))