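; BP_OnsetAnalyzer is an actor that pulses its cube's material on the onsets of a sound from an OnsetNRT analysis asset.
; BeginPlay assigns that sound to BP_SoundSource and loads channel 0's normalized onsets.
; Tick advances its own clock, sets strength to full as timestamps pass, decays it linearly, and writes it to the MI_Onset dynamic instance's Loudness parameter.
; Analyzed onset strengths do not scale the pulse.
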(event `self.ReceiveBeginPlay`
  (bind (_outonsettimestamps _outonsetstrengths) (`OnsetNRT.GetNormalizedChannelOnsetsBetweenTimes` (`self.OnsetNRT`) 0.0 (`self.Duration`) 0))
  (bind _sound (`AudioAnalyzerNRT.Sound` (`self.OnsetNRT`)))
  (`|ExecutionSequence`
    (:`then_0`
      ;[1 1 1] Initialize duration with the duration of the current sound being analyzed and set the sound inside the sound source
      (bind _returnvalue (`GameplayStatics.GetActorOfClass` "/Game/Sounds/BP_SoundSource.BP_SoundSource_C"))
      (`AudioComponent.SetSound` (`/Game/Sounds/BP_SoundSource.AudioComponent` _returnvalue) _sound)
      (set `self.Duration` (`SoundBase.Duration` _sound)))
    (:`then_1`
      ;[1 1 1] Initialize onsets timestamps and strengths
      (set `self.OnsetTimestamps` _outonsettimestamps)
      (set `self.OnsetStrengths` _outonsetstrengths))))

(event `self.ReceiveTick`
  (params (DeltaSeconds :type "Float (single-precision)"))
  (bind _currentonsetindex (`self.CurrentOnsetIndex`))
  ;[1 1 1] Only execute if onsets found
  (if (> (`KismetArrayLibrary.Array_Length` (`self.OnsetTimestamps`)) 0)
    (if (> (`KismetArrayLibrary.Array_Length` (`self.OnsetStrengths`)) 0)
      (`|ExecutionSequence`
        (:`then_0`
          ;[1 1 1] Detect onset
          (bind _output_get (set `self.CurrentTime` (+ (`self.CurrentTime`) DeltaSeconds)))
          ;[1 1 1] Set strengths
          (if (> _output_get (`|GetArrayItem` (`self.OnsetTimestamps`) (`self.CurrentOnsetIndex`)))
            (set `self.CurrentOnsetStrength` 1.0)
            ;[1 1 1] Advance index
            (if (< _currentonsetindex (- (`KismetArrayLibrary.Array_Length` (`self.OnsetTimestamps`)) 1))
              (`/Engine/EditorBlueprintResources/StandardMacros.IncrementInt` _currentonsetindex))))
        (:`then_1`
          ;[1 1 1] Decay
          (bind _output_get_2 (set `self.CurrentOnsetStrength` (- (`self.CurrentOnsetStrength`) (* (`self.DecaySpeed`) DeltaSeconds))))
          (if (< _output_get_2 0.0)
            (set `self.CurrentOnsetStrength` 0.0)))
        (:`then_2`
          ;[1 1 1] Set material parameter value
          (`MaterialInstanceDynamic.SetScalarParameterValue` (`self.Dynamic Material`) "Loudness" (`self.CurrentOnsetStrength`)))))))

(fn `UserConstructionScript`
  ;[1 1 1] Create and set dynamic material instance on the cube of this object
  (bind _returnvalue (`KismetMaterialLibrary.CreateDynamicMaterialInstance` "/Game/Materials/Instances/MI_Onset.MI_Onset"))
  (bind _output_get (set `self.Dynamic Material` _returnvalue))
  (`PrimitiveComponent.SetMaterial` (`self.Cube`) 0 _output_get))