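; BP_ConstantQAnalyzer is an audio visualizer that shows a ConstantQ NRT analysis as a row of red cubes, one per band.
; The construction script rebuilds the spaced cubes.
; BeginPlay plays the analyzed sound through BP_SoundSource, whose playback-percent callback samples normalized channel 0 values at the current time.
; Tick sets each cube's Z scale from its band, alongside unused frequency-range and averaging helpers.
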(event `self.ReceiveBeginPlay`
  (bind _soundsourceaudiocomponent (`self.SoundSourceAudioComponent`))
  (bind _sound (`AudioAnalyzerNRT.Sound` (`self.ConstantQNRT`)))
  (`|ExecutionSequence`
    (:`then_0`
      ;[1 1 1] Initialize duration with the duration of the current sound being analyzed and set the sound inside the sound source
      (bind _returnvalue (`GameplayStatics.GetActorOfClass` "/Game/Sounds/BP_SoundSource.BP_SoundSource_C"))
      (bind _output_get (set `self.SoundSourceAudioComponent` (`/Game/Sounds/BP_SoundSource.AudioComponent` _returnvalue)))
      (`AudioComponent.SetSound` _output_get _sound)
      (set `self.Duration` (`SoundBase.Duration` _sound)))
    (:`then_1`
      ;[1 1 1] Bind event to audio playback event
      (add `AudioComponent.OnAudioPlaybackPercent` _soundsourceaudiocomponent (delegate `OnAudioPlaybackPercent`))
      (`AudioComponent.Play` _soundsourceaudiocomponent 0.0))))

(event `OnAudioPlaybackPercent`
  (params (PlayingSoundWave :type "SoundWave Object Reference") (PlaybackPercent :type "Float (double-precision)"))
  ;[1 1 1] Get loudness result the NRT analyzer
  (set `self.CurrentConstantQ` (`ConstantQNRT.GetNormalizedChannelConstantQAtTime` (`self.ConstantQNRT`) (* PlaybackPercent (`self.Duration`)) 0)))

(event `self.ReceiveTick`
  (params (DeltaSeconds :type "Float (single-precision)"))
  ;[1 1 1] Update meshes of the analyzer
  (if (> (`KismetArrayLibrary.Array_Length` (`self.CurrentConstantQ`)) 0)
    (`self.UpdateMeshes`)))

(fn `GetFrequencyRange`
  (params (RangeIndex :type Integer))
  (returns (RequestedFrequencies :type "Array of Float (double-precision)"))
  (locals (CurrentFrequencies :type "Array of Float (double-precision)"))
  ;[1 1 1] Divides the frequencies in 3 and returns the requested part
  (if (or (> RangeIndex (- (`self.DivisionFactor`) 1)) (< RangeIndex 0))
    (return (`self.CurrentConstantQ`))
    (else
      (for _index (range (* (/ (`KismetArrayLibrary.Array_Length` (`self.CurrentConstantQ`)) (`self.DivisionFactor`)) RangeIndex) (+ (`KismetArrayLibrary.Array_Length` (`self.CurrentConstantQ`)) 1))
        (`KismetArrayLibrary.Array_Add` (`local.CurrentFrequencies`) (`|GetArrayItem` (`self.CurrentConstantQ`) _index)))
      (return (`local.CurrentFrequencies`)))))

(fn `GetFrequencyRangeAverage`
  (params (Frequencies :type "Array of Float (double-precision)"))
  (returns (Average :type "Float (double-precision)"))
  (locals (CurrentAverage :type "Float (double-precision)"))
  ;[1 1 1] Calculates the average for the given frequencies
  (for _array_element Frequencies
    (set `local.CurrentAverage` (+ (`local.CurrentAverage`) _array_element)))
  (return (/ (`local.CurrentAverage`) (`KismetMathLibrary.Conv_IntToDouble` (`KismetArrayLibrary.Array_Length` Frequencies)))))

(fn `UpdateMeshes`
  (bind (_startscale_x _startscale_y) (`KismetMathLibrary.BreakVector` (`self.StartScale`)))
  ;[1 1 1] Adjust scales of meshes depending on the frequencies
  (for (_array_element _array_index) (`self.Meshes`)
    (bind _output (`|GetArrayItem` (`self.CurrentConstantQ`) _array_index))
    (if (> _output 0.0)
      (bind (_returnvalue_x _returnvalue_y) (`KismetMathLibrary.BreakVector` (`SceneComponent.K2_GetComponentScale` _array_element)))
      (`SceneComponent.SetWorldScale3D` _array_element (`KismetMathLibrary.MakeVector` _returnvalue_x _returnvalue_y _output))
      (else
        (`SceneComponent.SetWorldScale3D` _array_element (`KismetMathLibrary.MakeVector` _startscale_x _startscale_y))))))

(fn `UserConstructionScript`
  (`|ExecutionSequence`
    (:`then_0`
      ;[1 1 1] Delete previous meshes
      (for _array_element (`self.Meshes`)
        (`ActorComponent.K2_DestroyComponent` _array_element))
      (`KismetArrayLibrary.Array_Clear` (`self.MeshTransforms`))
      (`KismetArrayLibrary.Array_Clear` (`self.Meshes`))
      (`KismetSystemLibrary.CollectGarbage`))
    (:`then_1`
      ;[1 1 1] Create transforms
      (for _index (range (`ConstantQNRTSettings.NumBands` (`ConstantQNRT.Settings` (`self.ConstantQNRT`))))
        (`KismetArrayLibrary.Array_Add` (`self.MeshTransforms`) (`KismetMathLibrary.MakeTransform` (* (`self.Spacing`) _index) (struct) (`self.StartScale`))))
      ;[1 1 1] Add components
      (for _array_element_2 (`self.MeshTransforms`)
        (bind _returnvalue (`AddComponent|NODE_AddStaticMeshComponent-1` :`RelativeTransform` _array_element_2))
        (`KismetArrayLibrary.Array_Add` (`self.Meshes`) _returnvalue))
      ;[1 1 1] Set static meshes
      (for _array_element_3 (`self.Meshes`)
        (`StaticMeshComponent.SetStaticMesh` _array_element_3 "/Engine/EngineMeshes/Cube.Cube")
        (`PrimitiveComponent.SetMaterial` _array_element_3 0 "/Game/Materials/Instances/MI_Red.MI_Red")))))