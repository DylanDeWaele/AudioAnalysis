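; Player controller that lets the player switch between controlling a human character and a drone.
; On BeginPlay it finds both actors in the level, and the ControlMode action flip-flops possession between them while setting IsDrone.
; Movement, look and jump inputs route to the active pawn based on that flag.
; Held Jump (in drone mode) and Crouch (in either mode) set flags that Tick uses to raise or lower the drone.
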(event `self.ReceiveBeginPlay`
  (`|ExecutionSequence`
    (:`then_0`
      (bind _returnvalue (`GameplayStatics.GetActorOfClass` "/Game/Player/BP_Player.BP_Player_C"))
      (set `self.PlayerRef` _returnvalue))
    (:`then_1`
      (bind _returnvalue_2 (`GameplayStatics.GetActorOfClass` "/Game/Player/BP_Drone.BP_Drone_C"))
      (set `self.DroneRef` _returnvalue_2))))

(event `InputAction|ControlMode`
  (params (Key :type "Key Structure"))
  ;[1 1 1] Toggle controlmode
  (:`Released`
    (`/Engine/EditorBlueprintResources/StandardMacros.FlipFlop`
      (:`A`
        (set `self.IsDrone` true)
        (`self.Possess` (`self.DroneRef`))
        (`KismetSystemLibrary.PrintString` "DRONE MODE ACTIVATED"))
      (:`B`
        (set `self.IsDrone` false)
        (`self.Possess` (`self.PlayerRef`))
        (`KismetSystemLibrary.PrintString` "HUMAN MODE ACTIVATED")))))

(event `InputAxis|MoveForward`
  (params (AxisValue :type "Float (single-precision)"))
  (bind _playerref (`self.PlayerRef`))
  ;[1 1 1] Forward movement
  (if (`self.IsDrone`)
    (`/Game/Player/BP_Drone.MoveForward` (`self.DroneRef`) AxisValue)
    (else
      (`Pawn.AddMovementInput` _playerref (`SceneComponent.GetForwardVector` (`Actor.RootComponent` _playerref)) AxisValue false))))

(event `InputAction|Jump`
  (params (Key :type "Key Structure"))
  ;[1 1 1] Flying or jumping
  (:`Pressed`
    (if (`self.IsDrone`)
      (set `self.SpaceHold` true)
      (else
        (`Character.Jump` (`self.PlayerRef`)))))
  (:`Released`
    (set `self.SpaceHold` false)))

(event `InputAxis|MoveRight`
  (params (AxisValue :type "Float (single-precision)"))
  (bind _playerref (`self.PlayerRef`))
  ;[1 1 1] Right movement
  (if (`self.IsDrone`)
    (`/Game/Player/BP_Drone.MoveRight` (`self.DroneRef`) AxisValue)
    (else
      (`Pawn.AddMovementInput` _playerref (`SceneComponent.GetRightVector` (`Actor.RootComponent` _playerref)) AxisValue false))))

(event `InputAction|Crouch`
  (params (Key :type "Key Structure"))
  ;[1 1 1] Flying down
  (:`Pressed`
    (set `self.CtrlHold` true))
  (:`Released`
    (set `self.CtrlHold` false)))

(event `InputAxis|LookUp`
  (params (AxisValue :type "Float (single-precision)"))
  ;[1 1 1] Mouse movement
  (if (`self.IsDrone`)
    (`Pawn.AddControllerPitchInput` (`self.DroneRef`) AxisValue)
    (else
      (`Pawn.AddControllerPitchInput` (`self.PlayerRef`) AxisValue))))

(event `self.ReceiveTick`
  (params (DeltaSeconds :type "Float (single-precision)"))
  (`|ExecutionSequence`
    (:`then_0`
      ;[1 1 1] Flying up
      (if (`self.CtrlHold`)
        (`/Game/Player/BP_Drone.MoveDown` (`self.DroneRef`))))
    (:`then_1`
      ;[1 1 1] Flying down
      (if (`self.SpaceHold`)
        (`/Game/Player/BP_Drone.MoveUp` (`self.DroneRef`))))))

(event `InputAxis|LookRight`
  (params (AxisValue :type "Float (single-precision)"))
  ;[1 1 1] Mouse movement
  (if (`self.IsDrone`)
    (`Pawn.AddControllerYawInput` (`self.DroneRef`) AxisValue)
    (else
      (`Pawn.AddControllerYawInput` (`self.PlayerRef`) AxisValue))))

(fn `UserConstructionScript`)