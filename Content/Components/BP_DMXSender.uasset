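; BP_DMXSender is a component that sends single-channel DMX values to universe 1 through the DMX subsystem.
; SendDMXValue computes the channel address from the base address, the frequency range index times the function amount, plus an offset.
; It maps a normalized value to the 0–255 byte range and sends it raw as a one-entry address-value map.
; The event graph has no active logic.
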(fn `SendDMXValue`
  (params (FrequencyRange :type Integer) (Offset :type Integer) (Value :type "Float (double-precision)"))
  ;[1 1 1] Send DMX value to certain address based on base address, function amount, frequency range and offset
  (`DMXSubsystem.SendDMXRaw` :`self` (subsystem `DMXSubsystem`) :`RemoteUniverse` 1 :`AddressValueMap` (`|MakeMap` (+ (+ (`self.BaseAddress`) (* FrequencyRange (`self.FunctionAmount`))) Offset) (`KismetMathLibrary.Conv_IntToByte` (`KismetMathLibrary.FTrunc` (`KismetMathLibrary.Lerp` 0.0 255.0 Value))))))