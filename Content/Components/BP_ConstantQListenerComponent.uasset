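; Actor component that gives audio-reactive values from a chosen frequency range, intended to drive effects like movement, dimmers and tilt.
; On BeginPlay it caches the level's BP_ConstantQAnalyzer, then queries it for the range's average, returning zero if none is valid.
; A normalized getter zeroes averages below a threshold and scales others against a running peak that only rises, amplifying small changes.
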(event `self.ReceiveBeginPlay`
  ;[1 1 1] Store constant Q analyzer
  (bind _returnvalue (`GameplayStatics.GetActorOfClass` "/Game/Analysis/ConstantQ/BP_ConstantQAnalyzer.BP_ConstantQAnalyzer_C"))
  (set `self.ConstantQAnalyzer` _returnvalue))

(fn `GetFrequencyRangeAverage`
  (returns (Average :type "Float (double-precision)"))
  (bind _constantqanalyzer (`self.ConstantQAnalyzer`))
  ;[1 1 1] Return the average of the chosen frequences
  (if (`KismetSystemLibrary.IsValid` _constantqanalyzer)
    (bind _requestedfrequencies (`/Game/Analysis/ConstantQ/BP_ConstantQAnalyzer.GetFrequencyRange` _constantqanalyzer (`self.FrequencyRange`)))
    (bind _average (`/Game/Analysis/ConstantQ/BP_ConstantQAnalyzer.GetFrequencyRangeAverage` _constantqanalyzer _requestedfrequencies))
    (return _average)
    (else
      (return 0.0))))

(fn `GetNormalizedFrequencyRangeAverage`
  (returns (NormalizedAverage :type "Float (double-precision)"))
  (bind _maxaverage (`self.MaxAverage`))
  ;[1 1 1] With this function the small changes of frequencies averages are scaled up so small changes will have larger effects on: movements, dimmers, tilt etc.
  (bind _average (`self.GetFrequencyRangeAverage`))
  (if (>= _average (`self.Treshold`))
    (if (> _average _maxaverage)
      (set `self.MaxAverage` _average)
      (bind _returnvalue (`KismetMathLibrary.NormalizeToRange` _average (`self.Treshold`) _maxaverage))
      (return _returnvalue)
      (else
        (return _returnvalue)))
    (else
      (return 0.0))))